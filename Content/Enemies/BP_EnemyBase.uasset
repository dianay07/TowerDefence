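; BP_EnemyBase is a base enemy Blueprint with an AbilitySystemComponent, tracking its travel along a line and handling death.
; Advance accumulates distance from delta times a GAS attribute.
; OnHealthChanged, without checking health, notifies EventManager of death, swaps spin for death sequence, then destroys the actor on a timer.
; The health check, debug prints and SetByCaller attribute initialization are disconnected.
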(event Custom|CustomEvent
  (Actor|DestroyActor))

(event Custom|DeathAnimation)

(event EventBeginPlay)

(event EventTick
  (params (DeltaSeconds :type Float%20%28single-precision%29)))

(event EventOnHealthChanged
  (params (OldValue :type Float%20%28single-precision%29) (NewValue :type Float%20%28single-precision%29))
  (Utilities|FlowControl|Sequence
    (:then_0
      (bind (_isvalid _eventmanager) (CallFunction|GetEventManager))
      (if _isvalid
        (Default|CallOnEnemyDied _eventmanager self)))
    (:then_1
      (Class|ActorSequenceComponent|StopSequence (Variables|Default|GetSpinSequence))
      (Class|ActorSequenceComponent|PlaySequence (Variables|Default|GetDeathSequence))
      (Utilities|Time|SetTimerbyEvent (delegate Custom|CustomEvent) 0.0))))

(fn ConstructionScript)

(fn Advance
  (params (Delta :type Float%20%28double-precision%29))
  ;[0.15 0.15 0.15 0.5] 적이 선상에서 얼마나 떨어져 있는지, 어디에 있는지 추적
  (bind _output_get (Variables|Default|SetDist (+ (* Delta (.ReturnValue (Class|AbilitySystemComponent|GetGameplayAttributeValue (Variables|Default|GetAbilitySystemComponent) "(AttributeName=\"MoveSpeed\",Attribute=/Script/TowerDefence.TDEnemySet:MoveSpeed,AttributeOwner=\"/Script/CoreUObject.Class'/Script/TowerDefence.TDEnemySet'\")"))) (Variables|Default|GetDist))))
  (return _output_get))
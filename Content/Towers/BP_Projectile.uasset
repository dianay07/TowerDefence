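; BP_Projectile is a tower projectile that homes in on its Target enemy and damages it on arrival.
; Each Tick, MoveTowardsTarget steps it toward the target's current location without sweeping and rotates it to face its travel direction.
; A hit is decided by distance, not collision: being very close, or farther than last frame to catch overshoot, calls OnHitTarget.
; It then applies damage and destroys itself, and also self-destructs if the target becomes invalid.
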(event EventBeginPlay)

(event Collision|EventActorBeginOverlap
  (params (OtherActor :type Actor%20Object%20Reference)))

(event EventTick
  (params (DeltaSeconds :type Float%20%28single-precision%29))
  (CallFunction|MoveTowardsTarget DeltaSeconds))

(fn ConstructionScript)

(fn MoveTowardsTarget
  (params (Delta :type Float%20%28double-precision%29))
  (bind _target (Variables|Default|GetTarget)
    (:then
      (bind _output_get (LocalVariables|SetDistance (Math|Vector|VectorLength (- (Transformation|GetActorLocation _target) (Transformation|GetActorLocation)))))
      (if (or (< _output_get 2e+01) (> _output_get (Variables|Default|GetLastDistance)))
        (CallFunction|OnHitTarget)
        (return)
        (else
          (bind _output_get_2 (LocalVariables|SetDirection (Math|Vector|Normalize (- (Transformation|GetActorLocation _target) (Transformation|GetActorLocation)))))
          (Transformation|SetActorLocation (+ (Transformation|GetActorLocation) (* _output_get_2 (* Delta (Variables|Default|GetSpeed)))) false false)
          ;[0.15 0.15 0.15 0.5] Target 방향으로 회전
          (Transformation|SetActorRotation (Math|Conversions|RotationFromXVector (LocalVariables|GetDirection)))
          (Variables|Default|SetLastDistance (LocalVariables|GetDistance)))))
    (:else
      (Actor|DestroyActor))))

(fn OnHitTarget
  (CallFunction|DamageEnemy (Variables|Default|GetTarget) (Variables|Default|GetDamage))
  (Actor|DestroyActor))
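; Catapult tower projectile that leaves a patch of sticky mud where it hits.
; OnHitTarget spawns a BP_StickyMud at the projectile's current location, passing along its Radius, then hands the new actor to BP_GameMode through PoolActor.
; The event graph holds only disabled stubs, and this Blueprint defines no movement or hit detection in its graphs.
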(event EventBeginPlay
  (|CallParentFunction) ; This node is disabled and will not be called.\nDrag off pins to build functionality.
)

(event Collision|EventActorBeginOverlap
  (params (OtherActor :type Actor%20Object%20Reference))
  (|CallParentFunction OtherActor) ; This node is disabled and will not be called.\nDrag off pins to build functionality.
)

(event EventTick
  (params (DeltaSeconds :type Float%20%28single-precision%29))
  (|CallParentFunction DeltaSeconds) ; This node is disabled and will not be called.\nDrag off pins to build functionality.
)

(fn ConstructionScript
  (|CallParentFunction))

(fn OnHitTarget
  (bind _returnvalue (Game|SpawnActorfromClass "/Game/Towers/BP_StickyMud.BP_StickyMud_C" (Math|Transform|MakeTransform (Transformation|GetActorLocation) "0, 0, 0" "1.000000,1.000000,1.000000") "Undefined" "MultiplyWithRoot" 0 (Variables|Default|GetRadius) 0))
  (bind _asbp_game_mode (Utilities|Casting|CastToBP_GameMode (Game|GetGameMode)))
  (Class|TDGameMode|PoolActor _asbp_game_mode _returnvalue))
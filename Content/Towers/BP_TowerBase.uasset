(event EventBeginPlay
  (bind _asbp_weapon (Utilities|Casting|CastToBP_Weapon (Variables|/Script/Engine.ChildActorComponent|GetChildActor (Variables|Default|GetChildActorWeapon))))
  (bind _output_get (Variables|Default|SetWeapon _asbp_weapon))
  (Variables|/Game/Towers/BP_Weapon.BP_Weapon_C|SetTower _output_get self)
  (CallFunction|GetTowerData))

(event Collision|EventActorBeginOverlap
  (params (OtherActor :type Actor%20Object%20Reference)))

(event EventTick
  (params (DeltaSeconds :type Float%20%28single-precision%29))
  (Abilities|TryActivateAbilitybyClass (Variables|Default|GetAbilitySystemComponent) (Variables|Default|GetDefaultAbility) true))

(event EventOnTowerAction
  (params (TowerAction :type ETowerActions%20Enum :default "None"))
  (CallFunction|DoTowerAction TowerAction))

(fn ConstructionScript)

(fn SetHighlight
  (params (IsHightlighted :type Boolean))
  (Rendering|SetVisibility (Variables|Default|GetHighlight) IsHightlighted true))

(fn Select
  (bind _output_get (LocalVariables|SetThisTowerActionTop (Variables|Default|GetTowerActionTop)))
  (Utilities|FlowControl|Sequence
    (:then_0
      (if (Utilities|Enum|Equal(Enum) _output_get "Upgrade")
        (bind _canupgrade (CallFunction|CanUpgrade))
        (if (not _canupgrade)
          (LocalVariables|SetThisTowerActionTop "None"))))
    (:then_1
      (bind _returnvalue (Game|SpawnActorfromClass "/Game/UI/BP_TowerActions.BP_TowerActions_C" (Math|Transform|MakeTransform (+ (Transformation|GetActorLocation) "0.000000,0.000000,100.000000") "0, 0, 0" "1.000000,1.000000,1.000000") "Undefined" "MultiplyWithRoot" self (LocalVariables|GetThisTowerActionTop) (Variables|Default|GetTowerActionLeft) (Variables|Default|GetTowerActionRight) (Variables|Default|GetTowerActionBottom) 0))
      (Variables|Default|SetBP_TowerActions _returnvalue))))

(fn UnSelect
  (bind _bp_toweractions (Variables|Default|GetBP_TowerActions)
    (:then
      (Actor|DestroyActor _bp_toweractions)
      (Variables|Default|SetBP_TowerActions 0))
    (:else)))

(fn DoTowerAction
  (params (TowerAction :type ETowerActions%20Enum :default "None"))
  (Utilities|FlowControl|Sequence
    (:then_0
      (bind _asbp_player (CallFunction|GetPlayer))
      (if true
        (Default|UnSelectTower _asbp_player)))
    (:then_1
      (bind _towercostorrefund (CallFunction|GetTowerDetails TowerAction))
      (bind _gamemode (CallFunction|GetGameMode))
      (if (Utilities|Enum|NotEqual(Enum) TowerAction "BreakDown")
        (bind _is_success (Default|SpendCoins _gamemode _towercostorrefund))
        (if _is_success
          _
          (else
            (return)))
        (else
          (Default|RefundCoins _gamemode _towercostorrefund)))
      (switch Utilities|FlowControl|Switch|SwitchonETowerActions TowerAction
        (:BuildTurret
          (LocalVariables|SetTowerClass "/Game/Towers/BP_TurretTower.BP_TurretTower_C"))
        (:BuildBallista
          (LocalVariables|SetTowerClass "/Game/Towers/BP_BallistaTower.BP_BallistaTower_C"))
        (:BuildCatapult
          (LocalVariables|SetTowerClass "/Game/Towers/BP_CatapultTower.BP_CatapultTower_C"))
        (:BuildCannon
          (LocalVariables|SetTowerClass "/Game/Towers/BP_CannonTower.BP_CannonTower_C"))
        (:Upgrade
          (CallFunction|UpgradeTower)
          (return))
        (:BreakDown
          (LocalVariables|SetTowerClass "BP_TowerBase_C"))))
    (:then_2
      (LocalVariables|GetTowerClass
        (:then
          (Game|SpawnActorfromClass (LocalVariables|GetTowerClass) (Transformation|GetActorTransform) "AlwaysSpawn" "MultiplyWithRoot" 0 0)
          (Actor|DestroyActor))
        (:else)))))

(fn GetRange
  (return (.ReturnValue (Class|AbilitySystemComponent|GetGameplayAttributeValue (Variables|Default|GetAbilitySystemComponent) "(AttributeName=\"Range\",Attribute=/Script/TowerDefence.TDTowerSet:Range,AttributeOwner=\"/Script/CoreUObject.Class'/Script/TowerDefence.TDTowerSet'\")"))))

(fn GetDamage
  (return (.ReturnValue (Class|AbilitySystemComponent|GetGameplayAttributeValue (Variables|Default|GetAbilitySystemComponent) "(AttributeName=\"Damage\",Attribute=/Script/TowerDefence.TDTowerSet:Damage,AttributeOwner=\"/Script/CoreUObject.Class'/Script/TowerDefence.TDTowerSet'\")"))))

(fn GetTowerData
  (Utilities|FlowControl|Sequence
    (:then_0
      (LocalVariables|SetIsDataValid false)
      (if (Utilities|Enum|NotEqual(Enum) (Variables|Default|GetType) "None")
        (bind (_isvalid _towermanager) (CallFunction|GetTowerManager))
        (if _isvalid
          (bind (_outtowerdata _returnvalue) (Class|TowerManager|GetTowerData _towermanager (Variables|Default|GetType)))
          (if _returnvalue
            (Variables|Default|SetTowerData _outtowerdata)
            (LocalVariables|SetIsDataValid true)))))
    (:then_1
      (if (LocalVariables|GetIsDataValid)
        (CallFunction|SetTowerAttributes (.range (Variables|Default|GetTowerData)) (.firerate (Variables|Default|GetTowerData)) (.damage (Variables|Default|GetTowerData)))))))

(fn GetRadius
  (return (.radius (Variables|Default|GetTowerData))))

(fn GetUpgradeCost
  (bind _towerdata (Variables|Default|GetTowerData))
  (Utilities|FlowControl|Sequence
    (:then_0
      (switch int (Variables|Default|GetUpgradeLevel)
        (:0
          (LocalVariables|SetTheCost (.upgradecost1 _towerdata)))
        (:1
          (LocalVariables|SetTheCost (.upgradecost2 _towerdata)))
        (:2
          (LocalVariables|SetTheCost (.upgradecost3 _towerdata)))))
    (:then_1
      (return (LocalVariables|GetTheCost)))))

(fn GetBreakdownRefund
  (bind _towerdata (Variables|Default|GetTowerData))
  (Utilities|FlowControl|Sequence
    (:then_0
      (LocalVariables|SetTheRefund (.buildcost _towerdata)))
    (:then_1
      (if (>= (Variables|Default|GetUpgradeLevel) 1)
        (LocalVariables|SetTheRefund (+ (LocalVariables|GetTheRefund) (.upgradecost1 _towerdata)))))
    (:then_2
      (if (>= (Variables|Default|GetUpgradeLevel) 2)
        (LocalVariables|SetTheRefund (+ (LocalVariables|GetTheRefund) (.upgradecost2 _towerdata)))))
    (:then_3
      (if (>= (Variables|Default|GetUpgradeLevel) 3)
        (LocalVariables|SetTheRefund (+ (LocalVariables|GetTheRefund) (.upgradecost3 _towerdata)))))
    (:then_4
      (return (LocalVariables|GetTheRefund)))))

(fn SetTowerAttributes
  (params (Range :type Float%20%28double-precision%29) (FireRate :type Float%20%28double-precision%29) (Damage :type Float%20%28double-precision%29))
  (bind _abilitysystemcomponent (Variables|Default|GetAbilitySystemComponent))
  (bind _returnvalue (Ability|GameplayEffect|AssignTagSetbyCallerMagnitude (GameplayEffects|MakeOutgoingSpec :self _abilitysystemcomponent :GameplayEffectClass "/Game/GAS/GE_TowerAttributes.GE_TowerAttributes_C") "(TagName=\"Tower.Range.SetByCaller\")" Range))
  (bind _returnvalue_2 (Ability|GameplayEffect|AssignTagSetbyCallerMagnitude _returnvalue "(TagName=\"Tower.FireRate.SetByCaller\")" FireRate))
  (bind _returnvalue_3 (Ability|GameplayEffect|AssignTagSetbyCallerMagnitude _returnvalue_2 "(TagName=\"Tower.Damage.SetByCaller\")" Damage))
  (GameplayEffects|ApplyGameplayEffectSpecToSelf _abilitysystemcomponent _returnvalue_3)
  (Development|PrintString (Utilities|String|Append "Range :" (Utilities|String|ToString(Float) Range) "FireRate: " (Utilities|String|ToString(Float) FireRate) "Damage :" (Utilities|String|ToString(Float) Damage))))

(fn CanUpgrade
  (return (< (Variables|Default|GetUpgradeLevel) 3)))

(fn UpgradeTower
  (bind _towerdata (Variables|Default|GetTowerData))
  (bind _canupgrade (CallFunction|CanUpgrade))
  (if _canupgrade
    (Math|Integer|IncrementInt (Variables|Default|GetUpgradeLevel)
      (:%20%20
        (LocalVariables|SetTowerRange (+ (* (* 0.5 (Variables|Default|GetUpgradeLevel)) (.range _towerdata)) (.range _towerdata)))
        (LocalVariables|SetTowerFireRate (+ (* (* 0.5 (Variables|Default|GetUpgradeLevel)) (.firerate _towerdata)) (.firerate _towerdata)))
        (LocalVariables|SetTowerDamage (+ (* (* 0.5 (Variables|Default|GetUpgradeLevel)) (.damage _towerdata)) (.damage _towerdata)))
        (CallFunction|SetTowerAttributes (LocalVariables|GetTowerRange) (LocalVariables|GetTowerFireRate) (LocalVariables|GetTowerDamage))))))

(fn GetTowerDetails
  (params (TowerAction :type ETowerActions%20Enum :default "None"))
  (Utilities|FlowControl|Sequence
    (:then_0
      (bind (_isvalid _towermanager) (CallFunction|GetTowerManager))
      (if _isvalid
        (LocalVariables|SetTowerManager _towermanager)
        (switch Utilities|FlowControl|Switch|SwitchonETowerActions TowerAction
          (:BuildTurret
            (bind (_outtowerdata _returnvalue) (Class|TowerManager|GetTowerData (LocalVariables|GetTowerManager) "Turret"))
            (if _returnvalue
              (LocalVariables|SetTheTowerData _outtowerdata)))
          (:BuildBallista
            (bind (_outtowerdata_2 _returnvalue_2) (Class|TowerManager|GetTowerData (LocalVariables|GetTowerManager) "Ballista"))
            (if _returnvalue_2
              (LocalVariables|SetTheTowerData _outtowerdata_2)))
          (:BuildCatapult
            (bind (_outtowerdata_3 _returnvalue_3) (Class|TowerManager|GetTowerData (LocalVariables|GetTowerManager) "Catapult"))
            (if _returnvalue_3
              (LocalVariables|SetTheTowerData _outtowerdata_3)))
          (:BuildCannon
            (bind (_outtowerdata_4 _returnvalue_4) (Class|TowerManager|GetTowerData (LocalVariables|GetTowerManager) "Cannon"))
            (if _returnvalue_4
              (LocalVariables|SetTheTowerData _outtowerdata_4)))
          (:Upgrade
            (bind _cost (CallFunction|GetUpgradeCost))
            (return _cost (Utilities|String|Append "Upgrade the" (.towername (Variables|Default|GetTowerData)) " 
for mo Power")))
          (:BreakDown
            (bind _refund (CallFunction|GetBreakdownRefund))
            (return _refund "Break Down")))
        (else
          (return 0 ""))))
    (:then_1
      (return (.buildcost (LocalVariables|GetTheTowerData)) (Utilities|String|Append "Back in my day, the 
" (.towername (LocalVariables|GetTheTowerData)) "brought all  
the enemies to the floor")))))
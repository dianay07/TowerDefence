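; BP_StickyMud is a short-lived tower-defense hazard that applies a sticky mud effect to enemies standing near it.
; It applies the debuff on spawn and again on a looping half-second timer until its lifespan expires a few seconds later.
; Each pulse asks the Wave Manager for enemies within a small radius and applies the GE_StickyMud Gameplay Effect through each enemy's Ability System Component.
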(event Custom|PulseStickyness
  (CallFunction|ApplyDebuff))

(event EventBeginPlay
  (Utilities|Time|SetTimerbyEvent (delegate Custom|PulseStickyness) 0.5 true)
  (CallFunction|ApplyDebuff)
  (Actor|SetLifeSpan 4.0))

(event Collision|EventActorBeginOverlap
  (params (OtherActor :type Actor%20Object%20Reference)))

(event EventTick
  (params (DeltaSeconds :type Float%20%28single-precision%29)))

(fn ConstructionScript)

(fn ApplyDebuff
  (bind (_isvalid _wavemanager) (CallFunction|GetWaveManager))
  (if _isvalid
    (bind _enemiesinrange (Default|GetEnemiesinRange _wavemanager (Transformation|GetActorLocation) 1e+02))
    (for _array_element _enemiesinrange
      (GameplayEffects|ApplyGameplayEffectToSelf :self (Ability|GetAbilitySystemComponent _array_element) :GameplayEffectClass "/Game/GAS/GE_StickyMud.GE_StickyMud_C"))))
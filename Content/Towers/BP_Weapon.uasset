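; Tower weapon actor that targets enemies and launches projectiles for its owning tower.
; Each tick it asks the wave manager for the furthest enemy in range and turns toward it, with a dev-mode CVar selecting normal or test variants.
; FireAtEnemy, not called within this Blueprint, takes a pooled projectile from the game mode at round-robin fire points and passes it target, damage and radius.
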(event EventBeginPlay)

(event Collision|EventActorBeginOverlap
  (params (OtherActor :type Actor%20Object%20Reference)))

(event EventTick
  (params (DeltaSeconds :type Float%20%28single-precision%29))
  (switch int (Class|TDFLUtility|GetCVarDevMode)
    (:0
      (CallFunction|FindEnemy)
      (CallFunction|FaceEnemy))
    (:1
      (CallFunction|FindEnemyforTest)
      (CallFunction|FaceEnemyforTest))))

(fn ConstructionScript)

(fn FindEnemy
  (bind (_isvalid _wavemanager) (CallFunction|GetWaveManagerC++))
  (if _isvalid
    (bind _returnvalue (Class|TDWaveManagerComponent|GetFurthestEnemy _wavemanager (Transformation|GetActorLocation) (Default|GetRange (Variables|Default|GetTower))))
    (bind _asbp_enemy_base (Utilities|Casting|CastToBP_EnemyBase _returnvalue))
    (Variables|Default|SetTarget _asbp_enemy_base)))

(fn FaceEnemy
  (bind _returnvalue (Transformation|GetActorLocation))
  (bind _target (Variables|Default|GetTarget))
  (bind _returnvalue_2 (Transformation|GetActorLocation _target))
  (Variables|Default|GetTarget
    (:then
      (Transformation|SetActorRotation (Math|Rotator|FindLookatRotation (Math|Vector|MakeVector (.x _returnvalue) (.y _returnvalue) 0.0) (Math|Vector|MakeVector (.x _returnvalue_2) (.y _returnvalue_2) 0.0))))
    (:else)))

(fn FireatEnemy
  (bind _tower (Variables|Default|GetTower))
  (Variables|Default|GetTarget
    (:then
      (bind (_location _rotation) (CallFunction|GetFirePoint))
      (bind _asbp_game_mode (Utilities|Casting|CastToBP_GameMode (Game|GetGameMode)))
      (bind _returnvalue (Class|TDGameMode|GetPoolActorfromClass _asbp_game_mode (Variables|Default|GetProjectileClass) (Math|Transform|MakeTransform _location _rotation "1.000000,1.000000,1.000000")))
      (bind _asbp_projectile (Utilities|Casting|CastToBP_Projectile _returnvalue))
      (LocalVariables|SetProjectile _asbp_projectile)
      (Utilities|FlowControl|Sequence
        (:then_0
          (Variables|/Game/Towers/BP_Projectile.BP_Projectile_C|SetTarget (LocalVariables|GetProjectile) (Variables|Default|GetTarget)))
        (:then_1
          (Variables|/Game/Towers/BP_Projectile.BP_Projectile_C|SetDamage (LocalVariables|GetProjectile) (Default|GetDamage _tower)))
        (:then_2
          (Variables|/Game/Towers/BP_Projectile.BP_Projectile_C|SetRadius (LocalVariables|GetProjectile) (Default|GetRadius _tower)))))
    (:else)))

(fn GetFirePoint
  (Utilities|FlowControl|Sequence
    (:then_0
      (if (not (< (Variables|Default|GetFirePointIndex) (Utilities|Array|Length (Variables|Default|GetFirePoints))))
        (Variables|Default|SetFirePointIndex 0)))
    (:then_1
      (LocalVariables|SetFirePoint (Utilities|Array|Get(acopy) (Variables|Default|GetFirePoints) (Variables|Default|GetFirePointIndex)))
      (Math|Integer|IncrementInt (Variables|Default|GetFirePointIndex)
        (:%20%20
          (bind _firepoint (LocalVariables|GetFirePoint)
            (:then
              (return (Transformation|GetWorldLocation _firepoint) (Transformation|GetWorldRotation _firepoint)))
            (:else
              (return (Transformation|GetActorLocation) (Transformation|GetActorRotation)))))))))

(fn FindEnemyforTest
  (bind (_isvalid _wavemanager) (CallFunction|GetWaveManagerC++))
  (if _isvalid
    (bind _returnvalue (Class|TDWaveManagerComponent|GetFurthestEnemy _wavemanager (Transformation|GetActorLocation) (+ (Class|TDTowerBase|GetRange (Variables|Default|GetTD_TowerBase)) 1e+02)))
    (if (Utilities|IsValid _returnvalue)
      (bind _asbp_enemy_base (Utilities|Casting|CastToBP_EnemyBase _returnvalue))
      (Variables|Default|SetTarget _asbp_enemy_base))))

(fn FaceEnemyforTest
  (bind _returnvalue (Transformation|GetActorLocation))
  (bind _target (Variables|Default|GetTarget))
  (bind _returnvalue_2 (Transformation|GetActorLocation _target))
  (Variables|Default|GetTarget
    (:then
      (Transformation|SetActorRotation (Math|Rotator|FindLookatRotation (Math|Vector|MakeVector (.x _returnvalue) (.y _returnvalue) 0.0) (Math|Vector|MakeVector (.x _returnvalue_2) (.y _returnvalue_2) 0.0))))
    (:else)))
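; Blueprint function library of shared helpers for the tower defense game.
; It provides typed getters for core framework objects and the wave manager, plus cursor traces that find towers or static mesh actors.
; DamageEnemy applies GE_Damage through GAS as a negated SetByCaller magnitude.
; Volume and video quality helpers read and write TDGameUserSettings, with volume changes also pushed live through a sound mix class override.
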(fn GetTowerUnderMouse
  (bind _returnvalue (Game|GetPlayerController 0))
  (bind _array (Utilities|Array|MakeArray "ObjectTypeQuery7"))
  (bind (_hitresult _returnvalue_2) (Class|PlayerController|GetHitResultUnderCursorforObjects _returnvalue _array true))
  (if _returnvalue_2
    (bind _asbp_tower_base (Utilities|Casting|CastToBP_TowerBase (.HitActor (Collision|BreakHitResult _hitresult)))
      (:then
        (return true _asbp_tower_base))
      (:CastFailed
        (return false 0)))
    (else
      (return false 0))))

(fn GetGameMode
  (bind _asbp_game_mode (Utilities|Casting|CastToBP_GameMode (Game|GetGameMode (LocalVariables|Get__WorldContext)))
    (:then
      (return _asbp_game_mode))
    (:CastFailed
      (Development|PrintString 0 "Failed to find BP_GameMode")
      (return 0))))

(fn GetPlayer
  (bind _asbp_player (Utilities|Casting|CastToBP_Player (Game|Player|GetPlayerPawn 0))
    (:then
      (return true _asbp_player))
    (:CastFailed
      (return false 0))))

(fn DamageEnemy
  (params (Enemy :type BP%20Enemy%20Base%20Object%20Reference) (Damage :type Float%20%28double-precision%29))
  (bind _returnvalue (Ability|GetAbilitySystemComponent Enemy))
  (bind _returnvalue_2 (Ability|GameplayEffect|AssignTagSetbyCallerMagnitude (GameplayEffects|MakeOutgoingSpec :self _returnvalue :GameplayEffectClass "/Game/GAS/GE_Damage.GE_Damage_C") "(TagName=\"Damage.SetByCaller\")" (* Damage -1.0)))
  (GameplayEffects|ApplyGameplayEffectSpecToSelf _returnvalue _returnvalue_2))

(fn GetWaveManager
  (bind _gamemode (CallFunction|GetGameMode))
  (return (Utilities|IsValid (Variables|/Game/Blueprints/BP_GameMode.BP_GameMode_C|GetWaveManager _gamemode)) 0))

(fn GetWaveManagerC++
  (bind _returnvalue (Class|TDFLUtility|GetWaveManager))
  (Utilities|IsValid _returnvalue
    (:Is%20Valid
      (return true _returnvalue))))

(fn GetGameInstance
  (bind _asbp_game_instance (Utilities|Casting|CastToBP_GameInstance (Game|GetGameInstance)))
  (return _asbp_game_instance))

(fn GetGameUserSettings
  (bind _returnvalue (Settings|GetGameUserSettings))
  (bind _astdgame_user_settings (Utilities|Casting|CastToTDGameUserSettings _returnvalue))
  (return _astdgame_user_settings))

(fn GetVolume
  (params (SoundClass :type Sound%20Class%20Object%20Reference))
  (bind _tdgame_user_settings (CallFunction|GetGameUserSettings))
  (LocalVariables|SetTD_GUS _tdgame_user_settings)
  (Utilities|FlowControl|Sequence
    (:then_0
      (if (== SoundClass "/Game/Audio/SC_Master.SC_Master")
        (return (Class|TDGameUserSettings|GetMasterVolume (LocalVariables|GetTD_GUS)))))
    (:then_1
      (if (== SoundClass "/Game/Audio/SC_Sound_Effects.SC_Sound_Effects")
        (return (Class|TDGameUserSettings|GetSoundEffectsVolume (LocalVariables|GetTD_GUS)))))
    (:then_2
      (if (== SoundClass "/Game/Audio/SC_Music.SC_Music")
        (return (Class|TDGameUserSettings|GetMusicVolume (LocalVariables|GetTD_GUS)))))))

(fn SetVolume
  (params (SoundClass :type Sound%20Class%20Object%20Reference) (Volume :type Float%20%28double-precision%29))
  (bind _tdgame_user_settings (CallFunction|GetGameUserSettings))
  (LocalVariables|SetTD_GUS _tdgame_user_settings)
  (Utilities|FlowControl|Sequence
    (:then_0
      (if (== SoundClass "/Game/Audio/SC_Master.SC_Master")
        (Class|TDGameUserSettings|SetMasterVolume (LocalVariables|GetTD_GUS) Volume)))
    (:then_1
      (if (== SoundClass "/Game/Audio/SC_Sound_Effects.SC_Sound_Effects")
        (Class|TDGameUserSettings|SetSoundEffectsVolume (LocalVariables|GetTD_GUS) Volume)))
    (:then_2
      (if (== SoundClass "/Game/Audio/SC_Music.SC_Music")
        (Class|TDGameUserSettings|SetMusicVolume (LocalVariables|GetTD_GUS) Volume)))
    (:then_3
      (Class|GameUserSettings|ApplyNonResolutionSettings (LocalVariables|GetTD_GUS))
      (Audio|SetSoundMixClassOverride 0 "/Game/Audio/SCM_Audio.SCM_Audio" SoundClass Volume 1.0 0.0 true)
      (Audio|PushSoundMixModifier 0 "/Game/Audio/SCM_Audio.SCM_Audio"))))

(fn GetVideoQuality
  (params (QualityOptionType :type EQualityOptionType%20Enum :default "None"))
  (bind _tdgame_user_settings (CallFunction|GetGameUserSettings))
  (LocalVariables|SetTD_GUS _tdgame_user_settings)
  (switch Utilities|FlowControl|Switch|SwitchonEQualityOptionType QualityOptionType
    (:Overall
      (return (Class|GameUserSettings|GetOverallScalabilityLevel (LocalVariables|GetTD_GUS))))
    (:ViewDistance
      (return (Class|GameUserSettings|GetViewDistanceQuality (LocalVariables|GetTD_GUS))))
    (:Shadow
      (return (Settings|GetShadowQuality (LocalVariables|GetTD_GUS))))
    (:GlobalIllumination
      (return (Settings|GetGlobalIlluminationQuality (LocalVariables|GetTD_GUS))))
    (:Reflections
      (return (Settings|GetReflectionQuality (LocalVariables|GetTD_GUS))))
    (:AntiAliasing
      (return (Class|GameUserSettings|GetAntiAliasingQuality (LocalVariables|GetTD_GUS))))
    (:Texture
      (return (Class|GameUserSettings|GetTextureQuality (LocalVariables|GetTD_GUS))))
    (:VisualEffect
      (return (Settings|GetVisualEffectQuality (LocalVariables|GetTD_GUS))))
    (:PostProcessing
      (return (Class|GameUserSettings|GetPostProcessingQuality (LocalVariables|GetTD_GUS))))
    (:Foliage
      (return (Class|GameUserSettings|GetFoliageQuality (LocalVariables|GetTD_GUS))))
    (:Shading
      (return (Class|GameUserSettings|GetShadingQuality (LocalVariables|GetTD_GUS))))))

(fn SetVideoQuality
  (params (QualityOptionType :type EQualityOptionType%20Enum :default "None") (QualityLevel :type Integer))
  (bind _tdgame_user_settings (CallFunction|GetGameUserSettings))
  (LocalVariables|SetTD_GUS _tdgame_user_settings)
  (Utilities|FlowControl|Sequence
    (:then_0
      (switch Utilities|FlowControl|Switch|SwitchonEQualityOptionType QualityOptionType
        (:Overall
          (Class|GameUserSettings|SetOverallScalabilityLevel (LocalVariables|GetTD_GUS) QualityLevel))
        (:ViewDistance
          (Class|GameUserSettings|SetViewDistanceQuality (LocalVariables|GetTD_GUS) QualityLevel))
        (:Shadow
          (Class|GameUserSettings|SetShadowQuality (LocalVariables|GetTD_GUS) QualityLevel))
        (:GlobalIllumination
          (Class|GameUserSettings|SetGlobalIlluminationQuality (LocalVariables|GetTD_GUS) QualityLevel))
        (:Reflections
          (Class|GameUserSettings|SetReflectionQuality (LocalVariables|GetTD_GUS) QualityLevel))
        (:AntiAliasing
          (Class|GameUserSettings|SetAntiAliasingQuality (LocalVariables|GetTD_GUS) QualityLevel))
        (:Texture
          (Class|GameUserSettings|SetTextureQuality (LocalVariables|GetTD_GUS) QualityLevel))
        (:VisualEffect
          (Class|GameUserSettings|SetVisualEffectQuality (LocalVariables|GetTD_GUS) QualityLevel))
        (:PostProcessing
          (Class|GameUserSettings|SetPostProcessingQuality (LocalVariables|GetTD_GUS) QualityLevel))
        (:Foliage
          (Class|GameUserSettings|SetFoliageQuality (LocalVariables|GetTD_GUS) QualityLevel))
        (:Shading
          (Class|GameUserSettings|SetShadingQuality (LocalVariables|GetTD_GUS) QualityLevel))))
    (:then_1
      (Class|GameUserSettings|ApplySettings (LocalVariables|GetTD_GUS) true))))

(fn GetStaticMeshUnderMouse
  (bind _returnvalue (Game|GetPlayerController 0))
  (bind _array (Utilities|Array|MakeArray "ObjectTypeQuery1"))
  (bind (_hitresult _returnvalue_2) (Class|PlayerController|GetHitResultUnderCursorforObjects _returnvalue _array true))
  (if _returnvalue_2
    (bind _as스태틱_메시_액터 (Utilities|Casting|CastToStaticMeshActor (.HitActor (Collision|BreakHitResult _hitresult)))
      (:then
        (return true _as스태틱_메시_액터))
      (:CastFailed
        (return false 0)))
    (else
      (return false 0))))

(fn GetTowerUnderMouseforTest
  (bind _returnvalue (Game|GetPlayerController 0))
  (bind _array (Utilities|Array|MakeArray "ObjectTypeQuery7"))
  (bind (_hitresult _returnvalue_2) (Class|PlayerController|GetHitResultUnderCursorforObjects _returnvalue _array true))
  (bind (_bblockinghit _binitialoverlap _time _distance _location _impactpoint _normal _impactnormal _physmat _hitactor) (Collision|BreakHitResult _hitresult))
  (if _returnvalue_2
    (bind _astd_bp_tower_base (Utilities|Casting|CastToTD_BP_TowerBase _hitactor)
      (:then
        (return true _astd_bp_tower_base))
      (:CastFailed
        (return false 0)))
    (else
      (return _bblockinghit 0))))
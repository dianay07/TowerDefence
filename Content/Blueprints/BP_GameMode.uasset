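; Game mode that holds the coin economy and heart health, and decides when the game is won or lost.
; On BeginPlay it spawns BP_EventManager, binding enemy deaths to coin rewards and enemy attacks to heart damage read from a gameplay attribute.
; Spend and refund functions broadcast coin changes through that manager.
; Depleted heart health means a loss and CheckIfWin queries WaveManager for remaining enemies; either result prints and pauses.
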(event EventBeginPlay
  (bind _returnvalue (Game|SpawnActorfromClass "/Game/Blueprints/BP_EventManager.BP_EventManager_C" (Math|Transform|MakeTransform "0, 0, 0" "0, 0, 0" "1.000000,1.000000,1.000000") "Undefined" "MultiplyWithRoot" 0 0))
  (bind _output_get (Variables|Default|SetEventManager _returnvalue))
  (EventDispatchers|BindEventtoOnEnemyDied _output_get (EventDispatchers|CreateEvent :!event OnEnemyDied))
  (EventDispatchers|BindEventtoOnEnemyAttacked _output_get (EventDispatchers|CreateEvent :!event OnEnemyAttacked)))

(event EventTick
  (params (DeltaSeconds :type Float%20%28single-precision%29)))

(fn ConstructionScript)

(fn OnEnemyDied
  (params (Enemy :type BP%20Enemy%20Base%20Object%20Reference))
  (Variables|Default|SetCoins (+ (Variables|/Game/Enemies/BP_EnemyBase.BP_EnemyBase_C|GetCoins Enemy) (Variables|Default|GetCoins)))
  (Default|CallOnCoinChanged (Variables|Default|GetEventManager) (Variables|Default|GetCoins) (Variables|Default|GetCoins)))

(fn HasCoins
  (params (Value :type Integer))
  (return (<= Value (Variables|Default|GetCoins))))

(fn SpendCoins
  (params (Values :type Integer))
  (bind _success (CallFunction|HasCoins Values))
  (if _success
    (Variables|Default|SetCoins (- (Variables|Default|GetCoins) Values))
    (Default|CallOnCoinChanged (Variables|Default|GetEventManager) (* Values -1) (Variables|Default|GetCoins))
    (return true)
    (else
      (return false))))

(fn RefundCoins
  (params (Values :type Integer))
  (Variables|Default|SetCoins (+ (Variables|Default|GetCoins) Values))
  (Default|CallOnCoinChanged (Variables|Default|GetEventManager) Values (Variables|Default|GetCoins))
  (return))

(fn OnEnemyAttacked
  (params (Enemy :type BP%20Enemy%20Base%20Object%20Reference))
  (bind _abilitysystemcomponent (Variables|/Script/TowerDefence.TDEnemyActor|GetAbilitySystemComponent Enemy))
  (bind (_bfound _returnvalue) (Class|AbilitySystemComponent|GetGameplayAttributeValue _abilitysystemcomponent "(AttributeName=\"Damage\",Attribute=/Script/TowerDefence.TDEnemySet:Damage,AttributeOwner=\"/Script/CoreUObject.Class'/Script/TowerDefence.TDEnemySet'\")"))
  (if _bfound
    (Variables|Default|SetHeartHealth (- (Variables|Default|GetHeartHealth) _returnvalue))
    (CallFunction|CheckifLoss)))

(fn GameEnded
  (params (IsWin :type Boolean))
  (Development|PrintString (Utilities|String|Append "Game Ended, but was it a Win?" (Utilities|String|ToString(Boolean) IsWin)))
  (Game|SetGamePaused true))

(fn CheckifWin
  (bind _enemiesremain (Default|DoEnemiesRemain (Variables|Default|GetWaveManager)))
  (if (not _enemiesremain)
    (CallFunction|GameEnded true)))

(fn CheckifLoss
  (if (<= (Variables|Default|GetHeartHealth) 0.0)
    (CallFunction|GameEnded false)))
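; Wave manager for a path-based enemy game that spawns timed waves, moves enemies along the Path and registers itself on the GameMode.
; Waves load from a DataTable; Tick counts down spawn delays, writing each copied struct back into the array.
; Enemies reaching the path end fire an attacked event and are destroyed; deaths, bound a tick after BeginPlay, trigger a win check.
; Also answers range, furthest-enemy and enemies-remaining queries.
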(event Custom|OneTimeInit
  (bind _eventmanager (CallFunction|GetEventManager))
  (if true
    (EventDispatchers|BindEventtoOnEnemyDied _eventmanager (EventDispatchers|CreateEvent :!event OnEnemyDied))))

(event EventBeginPlay
  (bind _path (Variables|Default|GetPath)
    (:then
      (bind _returnvalue (Default|GetLength _path))
      (Variables|Default|SetPathLength _returnvalue)
      (CallFunction|ImportData)
      (bind _gamemode (CallFunction|GetGameMode))
      (Variables|/Game/Blueprints/BP_GameMode.BP_GameMode_C|SetWaveManager _gamemode self)
      (Class|KismetSystemLibrary|SetTimerforNextTickDelegate (delegate Custom|OneTimeInit)))
    (:else)))

(event Collision|EventActorBeginOverlap
  (params (OtherActor :type Actor%20Object%20Reference)))

(event EventTick
  (params (DeltaSeconds :type Float%20%28single-precision%29))
  (CallFunction|UpdateWave DeltaSeconds))

(fn ConstructionScript)

(fn UpdateWave
  (params (Delta :type Float%20%28double-precision%29))
  (Utilities|FlowControl|Sequence
    (:then_0
      (CallFunction|AdvanceEnemies Delta))
    (:then_1
      (for (_array_element _array_index) (Variables|Default|GetWaveData)
        (if (> (Utilities|Time|GetGameTimeinSeconds) (.StartTime (Utilities|Struct|BreakWaveData _array_element)))
          (bind _output_get (LocalVariables|SetSpawnCount (.SpawnCount (Utilities|Struct|BreakWaveData _array_element))))
          (if (> _output_get 0)
            (LocalVariables|SetDelayRemaining (- (.DelayRemaining (Utilities|Struct|BreakWaveData _array_element)) Delta))
            (Utilities|FlowControl|Sequence
              (:then_0
                (if (<= (LocalVariables|GetDelayRemaining) 0.0)
                  (CallFunction|SpawnEnemy (.EnemyType (Utilities|Struct|BreakWaveData _array_element)))
                  (LocalVariables|SetDelayRemaining (.SpawnDeley (Utilities|Struct|BreakWaveData _array_element)))
                  (Math|Integer|DecrementInt (LocalVariables|GetSpawnCount))))
              (:then_1
                (Utilities|Array|SetArrayElem (Variables|Default|GetWaveData) _array_index (Utilities|Struct|MakeWaveData (.StartTime (Utilities|Struct|BreakWaveData _array_element)) (.EnemyType (Utilities|Struct|BreakWaveData _array_element)) (LocalVariables|GetSpawnCount) (.SpawnDeley (Utilities|Struct|BreakWaveData _array_element)) (LocalVariables|GetDelayRemaining)))))))))))

(fn AdvanceEnemies
  (params (Delta :type Float%20%28double-precision%29))
  (Utilities|FlowControl|Sequence
    (:then_0
      (for _array_element (Variables|Default|GetEnemies)
        (bind _distance (Default|Advance _array_element Delta))
        (if (< _distance (Variables|Default|GetPathLength))
          ;[0.15 0.15 0.15 0.5] 경로의 길이를 비교해서 이동
          (bind _location (Default|GetLocation (Variables|Default|GetPath) _distance))
          (Transformation|SetActorLocation _array_element _location false false)
          (else
            (Utilities|Array|Add (LocalVariables|GetExpiredEnemies) _array_element)))))
    (:then_1
      (for _array_element_2 (LocalVariables|GetExpiredEnemies)
        (Utilities|Array|RemoveItem (Variables|Default|GetEnemies) _array_element_2)
        (Utilities|FlowControl|Sequence
          (:then_0
            (bind (_isvalid _eventmanager) (CallFunction|GetEventManager))
            (if _isvalid
              (Default|CallOnEnemyAttacked _eventmanager _array_element_2) ; Called GameMode EnemyAttacked
            ))
          (:then_1
            (Actor|DestroyActor _array_element_2)))))))

(fn ImportData
  (bind _outrownames (DataTable|GetDataTableRowNames (Variables|Default|GetDataTable)))
  (for _array_element _outrownames
    (bind _returnvalue (Utilities|GetDataTableRow (Variables|Default|GetDataTable) _array_element)
      (:then
        (Utilities|Array|Add (Variables|Default|GetWaveData) _returnvalue)))))

(fn SpawnEnemy
  (params (EnemyType :type EEnemyType%20Enum :default "None"))
  (bind _enemytypeclass (Variables|Default|GetEnemyTypeClass))
  (bind (_value _returnvalue) (Utilities|Map|Find _enemytypeclass EnemyType))
  (if _returnvalue
    (bind _location (Default|GetLocation (Variables|Default|GetPath) 0.0))
    (bind _returnvalue_2 (Game|SpawnActorfromClass _value (Math|Transform|MakeTransform _location "0, 0, 0" "1.000000,1.000000,1.000000") "Undefined" "MultiplyWithRoot" 0 0))
    (Utilities|Array|Add (Variables|Default|GetEnemies) _returnvalue_2)))

(fn GetFurthestEnemy
  (params (Location :type Vector) (Radius :type Float%20%28double-precision%29))
  (for _array_element (Variables|Default|GetEnemies)
    ;[0.15 0.15 0.15 0.5] 타겟과 본인의 거리 계산후 지점 범위보다 가까우면
    (if (<= (Math|Vector|Distance2D(Vector) (Transformation|GetActorLocation _array_element) Location) Radius)
      (if (> (Variables|/Game/Enemies/BP_EnemyBase.BP_EnemyBase_C|GetDist _array_element) (LocalVariables|GetHitghDist))
        (LocalVariables|SetHitghDist (Variables|/Game/Enemies/BP_EnemyBase.BP_EnemyBase_C|GetDist _array_element))
        (LocalVariables|SetHighEenemy _array_element))))
  (return (LocalVariables|GetHighEenemy)))

(fn OnEnemyDied
  (params (Enemy :type BP%20Enemy%20Base%20Object%20Reference))
  (Utilities|Array|RemoveItem (Variables|Default|GetEnemies) Enemy)
  (bind _gamemode (CallFunction|GetGameMode))
  (Default|CheckifWin _gamemode)
  (Development|PrintString (Utilities|String|Append "On Enemy Died : " (Utilities|GetDisplayName Enemy))))

(fn GetEnemiesinRange
  (params (Location :type Vector) (Radius :type Float%20%28double-precision%29))
  (for _array_element (Variables|Default|GetEnemies)
    ;[0.15 0.15 0.15 0.5] 타겟과 본인의 거리 계산후 지점 범위보다 가까우면
    (if (<= (Math|Vector|Distance2D(Vector) (Transformation|GetActorLocation _array_element) Location) Radius)
      (Utilities|Array|Add (LocalVariables|GetTheEnemies) _array_element)))
  (return (LocalVariables|GetTheEnemies)))

(fn DoEnemiesRemain
  (if (Utilities|Array|IsEmpty (Variables|Default|GetEnemies))
    (for _array_element (Variables|Default|GetWaveData)
      (if (> (.SpawnCount (Utilities|Struct|BreakWaveData _array_element)) 0)
        (return true)))
    (return false)
    (else
      (return true))))
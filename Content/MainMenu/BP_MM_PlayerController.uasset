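; Main menu player controller that shows the main menu and opens its sub-screens.
; On BeginPlay it switches to UI-only input, shows the cursor, and adds WBP_MainMenu to the viewport.
; Options, save slot selection and credits functions each create their widget over the menu and store it in a shared WBPModal reference.
; OnMainMenu removes that modal widget and clears the reference.
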(event EventBeginPlay
  (Input|SetInputModeUIOnly self 0 "DoNotLock" false)
  (Variables|Default|SetbShowMouseCursor true)
  (bind _returnvalue (UserInterface|CreateWidget "/Game/MainMenu/WBP_MainMenu.WBP_MainMenu_C"))
  (bind _output_get (Variables|Default|SetWBP_MainMenu _returnvalue))
  (UserInterface|Viewport|AddtoViewport _output_get 0))

(event EventTick
  (params (DeltaSeconds :type Float%20%28single-precision%29)))

(fn ConstructionScript)

(fn OnOptions
  (bind _returnvalue (UserInterface|CreateWidget "/Game/MainMenu/WBP_Option.WBP_Option_C"))
  (bind _output_get (Variables|Default|SetWBP_Modal _returnvalue))
  (UserInterface|Viewport|AddtoViewport _output_get 0))

(fn OnSelectSaveSlot
  (bind _returnvalue (UserInterface|CreateWidget "/Game/MainMenu/WBP_SelectSaveSlot.WBP_SelectSaveSlot_C"))
  (bind _output_get (Variables|Default|SetWBP_Modal _returnvalue))
  (UserInterface|Viewport|AddtoViewport _output_get 0))

(fn OnCredits
  (bind _returnvalue (UserInterface|CreateWidget "/Game/MainMenu/WBP_Credits.WBP_Credits_C"))
  (bind _output_get (Variables|Default|SetWBP_Modal _returnvalue))
  (UserInterface|Viewport|AddtoViewport _output_get 0))

(fn OnMainMenu
  (bind _wbp_modal (Variables|Default|GetWBP_Modal)
    (:then
      (Widget|RemovefromParent _wbp_modal)
      (Variables|Default|SetWBP_Modal 0))
    (:else)))